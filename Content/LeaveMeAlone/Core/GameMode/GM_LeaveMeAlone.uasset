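; Game mode for LeaveMeAlone that runs the match countdown.
; On BeginPlay it starts a looping one-second timer that decrements GameTime and keeps the handle in TimeStop.
; When GameTime reaches exactly zero, it clears the timer and calls EventTimeStop to signal that time is up.
; Tick, the construction script and GameTimerStop1 contain no logic.
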(event Custom|CustomEvent
  (bind _output_get (Variables|Default|SetGame%20Time (- (Variables|Default|GetGame%20Time) 1)))
  (if (== _output_get 0)
    (Utilities|Time|ClearandInvalidateTimerbyHandle (Variables|Default|GetTime%20Stop))
    (Default|CallEventTimeStop)))

(event EventBeginPlay
  (bind _returnvalue (Utilities|Time|SetTimerbyEvent (delegate Custom|CustomEvent) 1.0 true))
  (Variables|Default|SetTime%20Stop _returnvalue))

(event EventTick
  (params (DeltaSeconds :type Float%20%28single-precision%29)))

(fn ConstructionScript)

(fn GameTimerStop1)