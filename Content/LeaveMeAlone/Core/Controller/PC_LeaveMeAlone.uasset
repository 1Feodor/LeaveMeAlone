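; Player controller for LeaveMeAlone that handles pausing and the victory and game-over screens.
; Pressing Pause stops weapon fire, pauses the game and shows the pause widget with UI-only input and a cursor.
; On BeginPlay it binds to the game mode's time-stop event for victory and the player's zero-health event for game over.
; Both outcomes pause the game and show their widget, with game over following a short delay.
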(event Custom|ZoreHealth_Event
  (Utilities|FlowControl|Delay 3.0)
  (Game|SetGamePaused true)
  (bind _returnvalue (UserInterface|CreateWidget "/Game/LeaveMeAlone/Widgets/UI/WBP_Game_Over.WBP_Game_Over_C"))
  (bind _output_get (Variables|Default|SetNewVar_0 _returnvalue))
  (UserInterface|Viewport|AddtoViewport _output_get 0)
  (Input|SetInputModeUIOnly self _output_get "DoNotLock" false)
  (Variables|Default|SetbShowMouseCursor true))

(event Custom|EventTimeStop_Event
  (Game|SetGamePaused true)
  (bind _returnvalue (UserInterface|CreateWidget "/Game/LeaveMeAlone/Widgets/UI/WBP_Victory.WBP_Victory_C"))
  (bind _output_get (Variables|Default|SetNewVar _returnvalue))
  (UserInterface|Viewport|AddtoViewport _output_get 0)
  (Input|SetInputModeUIOnly self _output_get "DoNotLock" false)
  (Variables|Default|SetbShowMouseCursor true))

(event EventBeginPlay
  (bind _returnvalue (Actor|GetActorOfClass "/Game/LeaveMeAlone/Core/GameMode/GM_LeaveMeAlone.GM_LeaveMeAlone_C"))
  (bind _output_get (Variables|Default|SetGM_LMA _returnvalue))
  (EventDispatchers|BindEventtoEventTimeStop _output_get (delegate Custom|EventTimeStop_Event))
  (bind _returnvalue_2 (Actor|GetActorOfClass "/Game/LeaveMeAlone/Core/Characters/CH_Player.CH_Player_C"))
  (bind _output_get_2 (Variables|Default|SetCH_P _returnvalue_2))
  (EventDispatchers|BindEventtoZoreHealth _output_get_2 (delegate Custom|ZoreHealth_Event)))

(event EventTick
  (params (DeltaSeconds :type Float%20%28single-precision%29)))

(event Input|ActionEvents|InputActionPause
  (params (Key :type Key%20Structure :default "None"))
  (:Pressed
    (if (not (Variables|Default|GetOnPause))
      (Variables|Default|SetOnPause true)
      (bind _returnvalue (Actor|GetActorOfClass "/Game/LeaveMeAlone/Weapon/A_Weapon.A_Weapon_C"))
      (Class|LMABaseWeapon|OffFire _returnvalue)
      (Game|SetGamePaused true)
      (bind _returnvalue_2 (UserInterface|CreateWidget "/Game/LeaveMeAlone/Widgets/UI/WBP_Pause.WBP_Pause_C"))
      (bind _output_get (Variables|Default|SetPauseWidget _returnvalue_2))
      (UserInterface|Viewport|AddtoViewport _output_get 0)
      (Input|SetInputModeUIOnly self _output_get "DoNotLock" false)
      (Variables|Default|SetbShowMouseCursor true))))

(fn ConstructionScript)

(fn CustomEvent)